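; BP_Award is a Character that handles the player's death and life count.
; On BeginPlay it moves the audio listener to its HeadLight and turns both lights red if GameOver returns true.
; The first damage it takes plays a death voice and ragdolls it.
; It then either decrements Life in AwardGameInstance and expires for a restart handled elsewhere, or opens the End level after a delay.
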(event `self.ReceiveBeginPlay`
  (bind _asbp_award_controller (cast `/Game/BP/BP_AwardController` (`self.GetController`))
    (:`then`
      (`PlayerController.SetAudioListenerOverride` :`self` _asbp_award_controller :`AttachToComponent` (`self.HeadLight`)))
    (:`CastFailed`
      _))
  (bind _isclear (`/Game/BP/MyFunctionLibrary.GameOver`))
  (if _isclear
    (`LightComponent.SetLightColor` (`self.HeadLight`) (struct :`R` 0.994792 :`A` 1.0) true)
    (`LightComponent.SetLightColor` (`self.PointLight`) (struct :`R` 0.994792 :`A` 1.0) true)))

(event `self.ReceiveAnyDamage`
  (params (Damage :type "Float (single-precision)") (DamageType :type "DamageType Object Reference") (InstigatedBy :type "Controller Object Reference") (DamageCauser :type "Actor Object Reference"))
  (bind _mesh (`self.Mesh`))
  (bind _asaward_game_instance (cast `/Game/BP/AwardGameInstance` (`GameplayStatics.GetGameInstance`) :!pure true))
  (bind _life (`/Game/BP/AwardGameInstance.Life` _asaward_game_instance))
  (`/Engine/EditorBlueprintResources/StandardMacros.DoOnce` false
    (:`Completed`
      (`GameplayStatics.PlaySound2D` "/Game/Audio/death_voice.death_voice")
      (`|ExecutionSequence`
        (:`then_0`
          ;[1 1 1] ラグドール化して動けないようにする
          (`CharacterMovementComponent.DisableMovement` (`self.CharacterMovement`))
          (`PrimitiveComponent.SetCollisionProfileName` _mesh "Ragdoll")
          (`PrimitiveComponent.SetSimulatePhysics` _mesh true))
        (:`then_1`
          ;[1 1 1] 残りLifeが1以上ならリスタート、そうでなければEnd画面遷移
          (if (> _life 0)
            (set `/Game/BP/AwardGameInstance.Life` (- _life 1) _asaward_game_instance)
            (`self.SetLifeSpan` 3.0)
            (else
              (`KismetSystemLibrary.Delay` 3.0)
              (`GameplayStatics.OpenLevel` "End"))))))))

(fn `UserConstructionScript`)