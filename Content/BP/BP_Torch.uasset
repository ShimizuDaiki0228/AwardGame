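; BP_Torch is a torch with a point light and a fire particle effect whose colour reflects goal and game-over state.
; The construction script tints the light and the FireColor particle parameter blue when IsGoal is set.
; BeginPlay calls GameOver once and, if it returns true, recolours both red, overriding any goal tint.
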(event `self.ReceiveBeginPlay`
  (bind _isclear (`/Game/BP/MyFunctionLibrary.GameOver`))
  (if _isclear
    (`LightComponent.SetLightColor` (`self.PointLight`) (struct :`R` 1.0 :`A` 1.0) true)
    (`ParticleSystemComponent.SetColorParameter` (`self.P_Fire`) "FireColor" (struct :`R` 1.0 :`A` 1.0))))

(fn `UserConstructionScript`
  (if (`self.IsGoal`)
    (`LightComponent.SetLightColor` (`self.PointLight`) (struct :`G` 0.256586 :`B` 1.0 :`A` 1.0) true)
    (`ParticleSystemComponent.SetColorParameter` (`self.P_Fire`) "FireColor" (struct :`G` 0.140875 :`B` 0.671875 :`A` 1.0))))